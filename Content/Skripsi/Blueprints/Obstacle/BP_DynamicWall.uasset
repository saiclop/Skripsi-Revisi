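; BP_DynamicWall is an obstacle actor: a maze wall between two cells that can open and close.
; Initialize stores both cells, direction and maze height, then SetOpen writes matching wall flags on opposite sides of both cells and clears their WallVisualize entries.
; A timeline lowers or raises the actor when animated; otherwise it snaps and records that state as the original, which Reset restores.
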(event Custom|SetOpen
  (params (open :type Boolean) (animate :type Boolean))
  (bind _returnvalue (Transformation|GetActorLocation))
  (bind _returnvalue_2 (Transformation|GetActorLocation))
  (bind _returnvalue_3 (Transformation|GetActorLocation))
  (bind _mazezloc (Variables|Default|GetmazeZLoc))
  (Variables|Default|Setopen open)
  (Variables|Default|Setanimating animate)
  (Utilities|FlowControl|Sequence
    (:then_0
      (switch Utilities|FlowControl|Switch|SwitchonEDirection (Variables|Default|Getdirection)
        (:Up
          (Utilities|Array|SetArrayElem (Variables|/Game/Skripsi/Blueprints/Maze/BP_Cell.BP_Cell_C|Getwall (Variables|Default|GetcurrentCell)) 0 (not (Variables|Default|Getopen)))
          (Utilities|Array|SetArrayElem (Variables|/Game/Skripsi/Blueprints/Maze/BP_Cell.BP_Cell_C|Getwall (Variables|Default|GetnextCell)) 2 (not (Variables|Default|Getopen)))
          (Utilities|Array|SetArrayElem (Variables|/Game/Skripsi/Blueprints/Maze/BP_Cell.BP_Cell_C|GetwallVisualize (Variables|Default|GetcurrentCell)) 0 false)
          (Utilities|Array|SetArrayElem (Variables|/Game/Skripsi/Blueprints/Maze/BP_Cell.BP_Cell_C|GetwallVisualize (Variables|Default|GetnextCell)) 2 false))
        (:Right
          (Utilities|Array|SetArrayElem (Variables|/Game/Skripsi/Blueprints/Maze/BP_Cell.BP_Cell_C|Getwall (Variables|Default|GetcurrentCell)) 1 (not (Variables|Default|Getopen)))
          (Utilities|Array|SetArrayElem (Variables|/Game/Skripsi/Blueprints/Maze/BP_Cell.BP_Cell_C|Getwall (Variables|Default|GetnextCell)) 3 (not (Variables|Default|Getopen)))
          (Utilities|Array|SetArrayElem (Variables|/Game/Skripsi/Blueprints/Maze/BP_Cell.BP_Cell_C|GetwallVisualize (Variables|Default|GetcurrentCell)) 1 false)
          (Utilities|Array|SetArrayElem (Variables|/Game/Skripsi/Blueprints/Maze/BP_Cell.BP_Cell_C|GetwallVisualize (Variables|Default|GetnextCell)) 3 false))
        (:Down
          (Utilities|Array|SetArrayElem (Variables|/Game/Skripsi/Blueprints/Maze/BP_Cell.BP_Cell_C|Getwall (Variables|Default|GetcurrentCell)) 2 (not (Variables|Default|Getopen)))
          (Utilities|Array|SetArrayElem (Variables|/Game/Skripsi/Blueprints/Maze/BP_Cell.BP_Cell_C|Getwall (Variables|Default|GetnextCell)) 0 (not (Variables|Default|Getopen)))
          (Utilities|Array|SetArrayElem (Variables|/Game/Skripsi/Blueprints/Maze/BP_Cell.BP_Cell_C|GetwallVisualize (Variables|Default|GetcurrentCell)) 2 false)
          (Utilities|Array|SetArrayElem (Variables|/Game/Skripsi/Blueprints/Maze/BP_Cell.BP_Cell_C|GetwallVisualize (Variables|Default|GetnextCell)) 0 false))
        (:Left
          (Utilities|Array|SetArrayElem (Variables|/Game/Skripsi/Blueprints/Maze/BP_Cell.BP_Cell_C|Getwall (Variables|Default|GetcurrentCell)) 3 (not (Variables|Default|Getopen)))
          (Utilities|Array|SetArrayElem (Variables|/Game/Skripsi/Blueprints/Maze/BP_Cell.BP_Cell_C|Getwall (Variables|Default|GetnextCell)) 1 (not (Variables|Default|Getopen)))
          (Utilities|Array|SetArrayElem (Variables|/Game/Skripsi/Blueprints/Maze/BP_Cell.BP_Cell_C|GetwallVisualize (Variables|Default|GetcurrentCell)) 3 false)
          (Utilities|Array|SetArrayElem (Variables|/Game/Skripsi/Blueprints/Maze/BP_Cell.BP_Cell_C|GetwallVisualize (Variables|Default|GetnextCell)) 1 false))))
    (:then_1
      (if (Variables|Default|Getanimating)
        (if (Variables|Default|Getopen)
          (bind _alpha (Timeline|WallAnimation PlayFromStart)
            (:Update
              (Transformation|SetActorLocation (Math|Vector|MakeVector (.x _returnvalue) (.y _returnvalue) (Math|Float|Lerp _mazezloc (+ _mazezloc -1e+02) _alpha)) false false))
            (:Finished
              (Variables|Default|Setanimating false)))
          (else
            (Timeline|WallAnimation ReverseFromEnd)))
        (else
          (Variables|Default|SetopenOri (Variables|Default|Getopen))
          (if (Variables|Default|Getopen)
            (Transformation|SetActorLocation (Math|Vector|MakeVector (.x _returnvalue_3) (.y _returnvalue_3) (+ (Variables|Default|GetmazeZLoc) -1e+02)) false false)
            (else
              (Transformation|SetActorLocation (Math|Vector|MakeVector (.x _returnvalue_2) (.y _returnvalue_2) (Variables|Default|GetmazeZLoc)) false false))))))))

(event EventBeginPlay
  (|CallParentFunction) ; This node is disabled and will not be called.\nDrag off pins to build functionality.
)

(event Collision|EventActorBeginOverlap
  (params (OtherActor :type Actor%20Object%20Reference))
  (|CallParentFunction OtherActor) ; This node is disabled and will not be called.\nDrag off pins to build functionality.
)

(event EventTick
  (params (DeltaSeconds :type Float%20%28single-precision%29))
  (|CallParentFunction DeltaSeconds) ; This node is disabled and will not be called.\nDrag off pins to build functionality.
)

(fn ConstructionScript
  (|CallParentFunction))

(fn Initialize
  (params (location :type Int%20Point%20Structure) (open :type Boolean) (direction :type EDirection%20Enum :default "Up") (currentCell :type BP%20Cell%20Object%20Reference%20%28by%20ref%29) (nextCell :type BP%20Cell%20Object%20Reference%20%28by%20ref%29) (nextLoc :type Int%20Point%20Structure) (mazeZLoc :type Float%20%28double-precision%29))
  (Variables|Default|Setlocation location)
  (Variables|Default|Setdirection direction)
  (Variables|Default|SetcurrentCell currentCell)
  (Variables|Default|SetnextCell nextCell)
  (Variables|Default|SetnextLocation nextLoc)
  (Variables|Default|SetmazeZLoc mazeZLoc)
  (CallFunction|SetOpen open false))

(fn Reset
  (CallFunction|SetOpen (Variables|Default|GetopenOri) false))