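; BP_Bomb is a countdown bomb obstacle that shows its remaining count on a text render.
; SetExplodeTime sets the count, and each external call to SubExplodeTime decrements it and updates the text while it stays above zero.
; At exactly zero it hides the bomb, shows the rock if any index is true in both wall arrays, and returns Explode and HasWall flags to the caller.
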(event EventBeginPlay
  (bind _outactors (Actor|GetAllActorsOfClass "/Script/Engine.CameraActor"))
  (Variables|Default|Setcamera (Utilities|Array|Get(acopy) _outactors)))

(event Collision|EventActorBeginOverlap
  (params (OtherActor :type Actor%20Object%20Reference)))

(event EventTick
  (params (DeltaSeconds :type Float%20%28single-precision%29)))

(fn ConstructionScript
  (|CallParentFunction))

(fn SubExplodeTime
  (params (walls :type Array%20of%20Booleans) (wallsVisualize :type Array%20of%20Booleans))
  (Math|Integer|DecrementInt (Variables|Default|GetexplodeTime)
    (:%20%20
      (if (> (Variables|Default|GetexplodeTime) 0)
        (Rendering|Components|TextRender|SetText (Variables|Default|GetTextRender) (Utilities|Text|ToText(Integer) (Variables|Default|GetexplodeTime)))
        (return false false)
        (elif (== (Variables|Default|GetexplodeTime) 0)
          (Rendering|SetVisibility (Variables|Default|GetBomb) false true)
          (bind (_array_element _array_index) (Utilities|Array|ForEachLoopwithBreak walls)
            (:LoopBody
              (if (and _array_element (Utilities|Array|Get(acopy) wallsVisualize _array_index))
                (Rendering|SetVisibility (Variables|Default|GetRock) true true)
                (return true true)))
            (:Completed
              (return true false)))
          (else
            (return false false)))))))

(fn SetExplodeTime
  (params (explodeTime :type Integer))
  (bind _output_get (Variables|Default|SetexplodeTime explodeTime))
  (Rendering|Components|TextRender|SetText (Variables|Default|GetTextRender) (Utilities|Text|ToText(Integer) _output_get)))