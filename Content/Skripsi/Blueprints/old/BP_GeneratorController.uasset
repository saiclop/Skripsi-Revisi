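; Controller that manages maze game generation across a set of save slots.
; GenerateNewGame deletes a game's slot, spawns a BP_GameGeneratorStruct to rebuild it, then loads a random available save into a new BP_Game.
; Generated_Event retries failed generations, loads a successful one if no game is active, and prints when all slots exist.
; BeginPlay is empty, leaving the startup fill-missing-slots logic disconnected.
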(event Custom|Generated_Event
  (params (success :type Boolean) (gameGenerator :type BP%20Game%20Generator%20Struct%20Object%20Reference))
  (Utilities|FlowControl|Sequence
    (:then_0
      (bind _complete (CallFunction|AllSaveCompleted?))
      (if _complete
        (Development|PrintString "COMPLETED")))
    (:then_1
      (if success
        (Variables|Default|Getgame
          (:then
            _)
          (:else
            (bind _returnvalue (Game|SpawnActorfromClass "/Game/Skripsi/Blueprints/BP_Game.BP_Game_C" (Math|Transform|MakeTransform "0, 0, 0" "0, 0, 0" "1.000000,1.000000,1.000000") "AlwaysSpawn" 0 0 0))
            (bind _output_get (Variables|Default|Setgame _returnvalue))
            (Default|LoadGameEvent _output_get (Variables|/Game/Skripsi/Blueprints/old/BP_GameGeneratorStruct.BP_GameGeneratorStruct_C|GetslotName gameGenerator))))
        (Actor|DestroyActor gameGenerator)
        (else
          (bind _returnvalue_2 (Game|SpawnActorfromClass "/Game/Skripsi/Blueprints/old/BP_GameGeneratorStruct.BP_GameGeneratorStruct_C" (Math|Transform|MakeTransform "0, 0, 0" "0, 0, 0" "1.000000,1.000000,1.000000") "AlwaysSpawn" 0 (Variables|/Game/Skripsi/Blueprints/old/BP_GameGeneratorStruct.BP_GameGeneratorStruct_C|GetmazeSize gameGenerator) (Variables|/Game/Skripsi/Blueprints/old/BP_GameGeneratorStruct.BP_GameGeneratorStruct_C|Getperfect gameGenerator) (Variables|/Game/Skripsi/Blueprints/old/BP_GameGeneratorStruct.BP_GameGeneratorStruct_C|GetslotName gameGenerator) self 0))
          (Actor|DestroyActor gameGenerator)
          (Default|NewGame _returnvalue_2))))))

(event Custom|GenerateNewGame
  (params (game :type BP%20Game%20Object%20Reference))
  (bind _slotname (Variables|/Game/Skripsi/Blueprints/BP_Game.BP_Game_C|GetslotName game))
  (SaveGame|DeleteGameinSlot _slotname)
  (bind _returnvalue (Game|SpawnActorfromClass "/Game/Skripsi/Blueprints/old/BP_GameGeneratorStruct.BP_GameGeneratorStruct_C" (Math|Transform|MakeTransform "0, 0, 0" "0, 0, 0" "1.000000,1.000000,1.000000") "AlwaysSpawn" 0 (Variables|Default|GetmazeSize) (Variables|Default|Getperfect) _slotname self 0))
  (Default|NewGame _returnvalue)
  (Actor|DestroyActor game)
  (bind (_available _unavailable) (CallFunction|CheckSaveGame))
  (Variables|Default|SetavailableSave _available)
  (Variables|Default|SetunavailableSave _unavailable)
  (if (Utilities|Array|IsNotEmpty (Variables|Default|GetavailableSave))
    (bind _returnvalue_2 (Game|SpawnActorfromClass "/Game/Skripsi/Blueprints/BP_Game.BP_Game_C" (Math|Transform|MakeTransform "0, 0, 0" "0, 0, 0" "1.000000,1.000000,1.000000") "AlwaysSpawn" 0 0 0))
    (bind _output_get (Variables|Default|Setgame _returnvalue_2))
    (Default|LoadGameEvent _output_get (Utilities|Array|Get(acopy) (Variables|Default|GetavailableSave) (Math|Random|RandomIntegerinRange 0 (Utilities|Array|LastIndex (Variables|Default|GetavailableSave)))))))

(event EventBeginPlay)

(fn ConstructionScript)

(fn CheckSaveGame
  (for _array_element (Variables|Default|GetsaveSlotNames)
    (bind _returnvalue (SaveGame|DoesSaveGameExist _array_element))
    (if _returnvalue
      (Utilities|Array|Add (LocalVariables|GetL_available) _array_element)
      (else
        (Utilities|Array|Add (LocalVariables|GetL_unavailable) _array_element))))
  (return (LocalVariables|GetL_available) (LocalVariables|GetL_unavailable)))

(fn AllSaveCompleted?
  (for _array_element (Variables|Default|GetsaveSlotNames)
    (bind _returnvalue (SaveGame|DoesSaveGameExist _array_element))
    (if (not _returnvalue)
      (return false)))
  (return true))