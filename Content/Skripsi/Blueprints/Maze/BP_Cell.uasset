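; BP_Cell is a maze cell actor that builds and clears the walls on its four edges.
; GenerateWall spawns a rotated, scaled BP_Wall on each edge where both Wall and WallVisualize are true, positioned from the cell's Size.
; It spawns walls at local offsets, then attaches them with KeepRelative to land on the cell, storing them in BPWall.
; RemoveWall destroys those actors and empties the array.
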(event EventBeginPlay)

(fn ConstructionScript)

(fn GenerateWall
  (Utilities|FlowControl|Sequence
    (:then_0
      (if (and (Utilities|Array|Get(acopy) (Variables|Default|GetwallVisualize)) (Utilities|Array|Get(acopy) (Variables|Default|Getwall)))
        (bind _returnvalue (Game|SpawnActorfromClass "/Game/Skripsi/Blueprints/Maze/BP_Wall.BP_Wall_C" (Math|Transform|MakeTransform (+ "0.000000,0.000000,50.000000" (Math|Vector|MakeVector (* (Variables|Default|Getsize) 0.5) 0.0 0.0)) "0.000000,180.000000,0.000000" "0.500000,1.000000,1.000000") "Undefined" 0 0))
        (Utilities|Array|Add (Variables|Default|GetBP_Wall) _returnvalue)
        (Transformation|AttachComponentToComponent _returnvalue (Variables|Default|GetDefaultSceneRoot) "None" "KeepRelative" "KeepRelative" "KeepRelative" true)))
    (:then_1
      (if (and (Utilities|Array|Get(acopy) (Variables|Default|GetwallVisualize) 1) (Utilities|Array|Get(acopy) (Variables|Default|Getwall) 1))
        (bind _returnvalue_2 (Game|SpawnActorfromClass "/Game/Skripsi/Blueprints/Maze/BP_Wall.BP_Wall_C" (Math|Transform|MakeTransform (+ "0.000000,0.000000,50.000000" (Math|Vector|MakeVector (Math|Conversions|ToFloat(Integer) (Variables|Default|Getsize)) (* (Variables|Default|Getsize) 0.5) 0.0)) "0.000000,-90.000000,0.000000" "0.500000,1.000000,1.000000") "Undefined" 0 0))
        (Utilities|Array|Add (Variables|Default|GetBP_Wall) _returnvalue_2)
        (Transformation|AttachComponentToComponent _returnvalue_2 (Variables|Default|GetDefaultSceneRoot) "None" "KeepRelative" "KeepRelative" "KeepRelative" true)))
    (:then_2
      (if (and (Utilities|Array|Get(acopy) (Variables|Default|GetwallVisualize) 2) (Utilities|Array|Get(acopy) (Variables|Default|Getwall) 2))
        (bind _returnvalue_3 (Game|SpawnActorfromClass "/Game/Skripsi/Blueprints/Maze/BP_Wall.BP_Wall_C" (Math|Transform|MakeTransform (+ "0.000000,0.000000,50.000000" (Math|Vector|MakeVector (* (Variables|Default|Getsize) 0.5) (Math|Conversions|ToFloat(Integer) (Variables|Default|Getsize)) 0.0)) "0, 0, 0" "0.500000,1.000000,1.000000") "Undefined" 0 0))
        (Utilities|Array|Add (Variables|Default|GetBP_Wall) _returnvalue_3)
        (Transformation|AttachComponentToComponent _returnvalue_3 (Variables|Default|GetDefaultSceneRoot) "None" "KeepRelative" "KeepRelative" "KeepRelative" true)))
    (:then_3
      (if (and (Utilities|Array|Get(acopy) (Variables|Default|GetwallVisualize) 3) (Utilities|Array|Get(acopy) (Variables|Default|Getwall) 3))
        (bind _returnvalue_4 (Game|SpawnActorfromClass "/Game/Skripsi/Blueprints/Maze/BP_Wall.BP_Wall_C" (Math|Transform|MakeTransform (+ "0.000000,0.000000,50.000000" (Math|Vector|MakeVector 0.0 (* (Variables|Default|Getsize) 0.5) 0.0)) "0.000000,90.000000,0.000000" "0.500000,1.000000,1.000000") "Undefined" 0 0))
        (Utilities|Array|Add (Variables|Default|GetBP_Wall) _returnvalue_4)
        (Transformation|AttachComponentToComponent _returnvalue_4 (Variables|Default|GetDefaultSceneRoot) "None" "KeepRelative" "KeepRelative" "KeepRelative" true)))))

(fn RemoveWall
  (bind _bp_wall (Variables|Default|GetBP_Wall))
  (for _array_element _bp_wall
    (Actor|DestroyActor _array_element))
  (Utilities|Array|Clear _bp_wall))