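; Enemy NPC for a grid maze that steps one cell at a time toward the player, inheriting from a parent NPC class.
; Move tries the preferred Horizontal or Vertical axis first, falls back to the other when blocked or aligned, then walks via AI MoveTo.
; BombExplode knocks it back one cell opposite its last Direction through FlyEvent.
; Despite the Attacker name, CanAttack? always returns false here.
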(event Custom|MoveEvent
  (params (cells :type Array%20of%20BP%20Cell%20Object%20References) (mazeSize :type Int%20Point%20Structure) (gridSize :type Integer) (playerLoc :type Int%20Point%20Structure))
  (bind _returnvalue (/ gridSize 2))
  (bind _returnvalue_2 (Math|Conversions|ToFloat(Integer) _returnvalue))
  (if (not (Variables|Default|Getdied))
    (Variables|Default|Setmoving true)
    (Variables|Default|SetmoveCell false)
    (Utilities|FlowControl|Sequence
      (:then_0
        (switch Utilities|FlowControl|Switch|SwitchonEMovementPriority (Variables|Default|Getmovement)
          (:Horizontal
            (if (and (> (.x playerLoc) (.x (Variables|Default|Getlocation))) (not (Utilities|Array|Get(acopy) (Variables|/Game/Skripsi/Blueprints/Maze/BP_Cell.BP_Cell_C|Getwall (Utilities|Array|Get(acopy) cells (CallFunction|GetIndex (Variables|Default|Getlocation) mazeSize))) 1))) :!label _label
              (Variables|Default|Setlocation (Utilities|Struct|MakeIntPoint (+ (.x (Variables|Default|Getlocation)) 1) (.y (Variables|Default|Getlocation))))
              (Variables|Default|SetmoveCell true)
              (Variables|Default|Setdirection "NewEnumerator1")
              (elif (and (< (.x playerLoc) (.x (Variables|Default|Getlocation))) (not (Utilities|Array|Get(acopy) (Variables|/Game/Skripsi/Blueprints/Maze/BP_Cell.BP_Cell_C|Getwall (Utilities|Array|Get(acopy) cells (CallFunction|GetIndex (Variables|Default|Getlocation) mazeSize))) 3)))
                (Variables|Default|Setlocation (Utilities|Struct|MakeIntPoint (+ (.x (Variables|Default|Getlocation)) -1) (.y (Variables|Default|Getlocation))))
                (Variables|Default|SetmoveCell true)
                (Variables|Default|Setdirection "NewEnumerator3")
                (else
                  (switch Utilities|FlowControl|Switch|SwitchonEMovementPriority (Variables|Default|Getmovement)
                    (:Horizontal
                      (if (and (< (.y playerLoc) (.y (Variables|Default|Getlocation))) (not (Utilities|Array|Get(acopy) (Variables|/Game/Skripsi/Blueprints/Maze/BP_Cell.BP_Cell_C|Getwall (Utilities|Array|Get(acopy) cells (CallFunction|GetIndex (Variables|Default|Getlocation) mazeSize)))))) :!label _label_2
                        (Variables|Default|Setlocation (Utilities|Struct|MakeIntPoint (.x (Variables|Default|Getlocation)) (+ (.y (Variables|Default|Getlocation)) -1)))
                        (Variables|Default|SetmoveCell true)
                        (Variables|Default|Setdirection "NewEnumerator0")
                        (elif (and (> (.y playerLoc) (.y (Variables|Default|Getlocation))) (not (Utilities|Array|Get(acopy) (Variables|/Game/Skripsi/Blueprints/Maze/BP_Cell.BP_Cell_C|Getwall (Utilities|Array|Get(acopy) cells (CallFunction|GetIndex (Variables|Default|Getlocation) mazeSize))) 2)))
                          (Variables|Default|Setlocation (Utilities|Struct|MakeIntPoint (.x (Variables|Default|Getlocation)) (+ (.y (Variables|Default|Getlocation)) 1)))
                          (Variables|Default|SetmoveCell true)
                          (Variables|Default|Setdirection "NewEnumerator2")
                          (else
                            (switch Utilities|FlowControl|Switch|SwitchonEMovementPriority (Variables|Default|Getmovement)
                              (:Vertical
                                (goto _label))))))))))))
          (:Vertical
            (goto _label_2))))
      (:then_1
        (if (Variables|Default|GetmoveCell)
          (AI|AIMoveTo self (+ (Transformation|GetActorLocation (Utilities|Array|Get(acopy) cells (CallFunction|GetIndex (Variables|Default|Getlocation) mazeSize))) (Math|Vector|MakeVector _returnvalue_2 _returnvalue_2 0.0)) 0 5.0 true
            (:OnSuccess
              (Variables|Default|Setmoving false)))
          (else
            (Variables|Default|Setmoving false)))))))

(event EventBeginPlay)

(fn ConstructionScript
  (|CallParentFunction)
  (Variables|Default|Setdirection "NewEnumerator4"))

(fn CanAttack?
  (params (playerLocation :type Int%20Point%20Structure) (cells :type Array%20of%20BP%20Cell%20Object%20References) (mazeSize :type Int%20Point%20Structure))
  (return false))

(fn SetMovement
  (params (movement :type EMovementPriority%20Enum :default "Horizontal"))
  (Variables|Default|Setmovement movement))

(fn BombExplode
  (params (cells :type Array%20of%20BP%20Cell%20Object%20References) (mazeSize :type Int%20Point%20Structure) (gridSize :type Integer))
  (bind _returnvalue (/ gridSize 2))
  (bind _returnvalue_2 (Math|Conversions|ToFloat(Integer) _returnvalue))
  (|CallParentFunction cells mazeSize gridSize)
  (switch Utilities|FlowControl|Switch|SwitchonE_Direction (Variables|Default|Getdirection)
    (:NewEnumerator0
      (Variables|Default|Setlocation (Utilities|Struct|MakeIntPoint (.x (Variables|Default|Getlocation)) (+ (.y (Variables|Default|Getlocation)) 1))))
    (:NewEnumerator1
      (Variables|Default|Setlocation (Utilities|Struct|MakeIntPoint (+ (.x (Variables|Default|Getlocation)) -1) (.y (Variables|Default|Getlocation)))))
    (:NewEnumerator2
      (Variables|Default|Setlocation (Utilities|Struct|MakeIntPoint (.x (Variables|Default|Getlocation)) (+ (.y (Variables|Default|Getlocation)) -1))))
    (:NewEnumerator3
      (Variables|Default|Setlocation (Utilities|Struct|MakeIntPoint (+ (.x (Variables|Default|Getlocation)) 1) (.y (Variables|Default|Getlocation))))))
  (CallFunction|FlyEvent (+ (Transformation|GetActorLocation (Utilities|Array|Get(acopy) cells (CallFunction|GetIndex (Variables|Default|Getlocation) mazeSize))) (Math|Vector|MakeVector _returnvalue_2 _returnvalue_2 0.0))))

(fn Destroy
  (|CallParentFunction)
  (Actor|DestroyActor))

(fn Move
  (params (cells :type Array%20of%20BP%20Cell%20Object%20References) (mazeSize :type Int%20Point%20Structure) (gridSize :type Integer) (playerLoc :type Int%20Point%20Structure))
  (|CallParentFunction cells mazeSize gridSize playerLoc)
  (CallFunction|MoveEvent cells mazeSize gridSize playerLoc))