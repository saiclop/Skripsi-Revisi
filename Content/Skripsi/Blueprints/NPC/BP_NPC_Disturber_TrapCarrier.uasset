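; Trap-carrier variant of a disturber NPC that places a landmine as its obstacle, extending its parent class's behavior.
; SpawnObstacle hides the static mesh, spawns a BP_Landmine at the given location regardless of collision, and stores it as Obstacle.
; ResetPosition destroys that obstacle if still valid and only then shows the mesh again.
; The construction script sets Power, and BeginPlay only calls the parent.
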(event EventBeginPlay
  (|CallParentFunction))

(event Collision|EventActorBeginOverlap
  (params (OtherActor :type Actor%20Object%20Reference))
  (|CallParentFunction OtherActor) ; This node is disabled and will not be called.\nDrag off pins to build functionality.
)

(event EventTick
  (params (DeltaSeconds :type Float%20%28single-precision%29))
  (|CallParentFunction DeltaSeconds) ; This node is disabled and will not be called.\nDrag off pins to build functionality.
)

(fn ConstructionScript
  (|CallParentFunction)
  (Variables|Default|Setpower 1))

(fn SpawnObstacle
  (params (location :type Vector :default "0, 0, 0"))
  (|CallParentFunction location)
  (Rendering|SetVisibility (Variables|Default|GetStaticMesh) false false)
  (bind _returnvalue (Game|SpawnActorfromClass "/Game/Skripsi/Blueprints/Obstacle/BP_Landmine.BP_Landmine_C" (Math|Transform|MakeTransform location "0, 0, 0" "1.000000,1.000000,1.000000") "AlwaysSpawn" 0 0))
  (Variables|Default|Setobstacle _returnvalue))

(fn ResetPosition
  (params (location :type Vector :default "0, 0, 0"))
  (bind _obstacle (Variables|Default|Getobstacle))
  (|CallParentFunction location)
  (Utilities|IsValid _obstacle
    (:Is%20Valid
      (Actor|DestroyActor _obstacle)
      (Rendering|SetVisibility (Variables|Default|GetStaticMesh) true false))))