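; Maze NPC that walks a stored cell path and can spawn an obstacle, with SpawnObstacle left empty here.
; Extends parent NPC actions with AI moves that wait if the player occupies the next cell, and records the obstacle position on reaching its cell.
; Bomb blasts fly it back along the original path.
; Montage-timed events clear attack, death and spawn flags; death and spawning sink it below the level.
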(event Custom|DieEvent
  (Utilities|FlowControl|Delay 0.3)
  (bind _returnvalue (Animation|PlayAnimMontage "/Game/Asset/Goblin/Animations/Anim_Lose_Montage.Anim_Lose_Montage" 1.0 "None"))
  (Utilities|FlowControl|Delay (- _returnvalue 0.1))
  (Transformation|SetActorLocation "0.000000,0.000000,-250.000000" false false)
  (Variables|Default|Setdying false))

(event Custom|MoveEvent
  (params (cells :type Array%20of%20BP%20Cell%20Object%20References) (mazeSize :type Int%20Point%20Structure) (gridSize :type Integer) (playerLoc :type Int%20Point%20Structure))
  (bind _returnvalue (/ gridSize 2))
  (bind _path (Variables|Default|Getpath))
  (bind _returnvalue_2 (Math|Conversions|ToFloat(Integer) _returnvalue))
  (bind _output (Utilities|Array|Get(acopy) _path))
  (if (not (Variables|Default|Getdied))
    (Variables|Default|Setmoving true)
    (if (Class|KismetMathLibrary|EqualIntPointIntPoint playerLoc (Utilities|Array|Get(acopy) (Variables|Default|Getpath)))
      (Variables|Default|Setmoving false)
      (else
        (Variables|Default|Setlocation _output)
        (Variables|Default|Setvector (+ (Transformation|GetActorLocation (Utilities|Array|Get(acopy) cells (CallFunction|GetIndex _output mazeSize))) (Math|Vector|MakeVector _returnvalue_2 _returnvalue_2 0.0)))
        (AI|AIMoveTo self (Variables|Default|Getvector) 0 5.0 true
          (:OnSuccess
            (Utilities|Array|RemoveIndex (Variables|Default|Getpath))
            (Utilities|FlowControl|Sequence
              (:then_0
                (if (Class|KismetMathLibrary|EqualIntPointIntPoint (Variables|Default|Getlocation) (Variables|Default|GetobstacleLocation))
                  (Variables|Default|SetobstacleVectorLoc (Variables|Default|Getvector))))
              (:then_1
                (Variables|Default|Setmoving false)))))))))

(event Custom|SpawnObstacleEvent
  (Variables|Default|Setspawning true)
  (bind _returnvalue (Animation|PlayAnimMontage "/Game/Asset/Goblin/Animations/Anim_Agr_Montage.Anim_Agr_Montage" 1.0 "None"))
  (Utilities|FlowControl|Delay _returnvalue)
  (CallFunction|SpawnObstacle (Variables|Default|GetobstacleVectorLoc))
  (Variables|Default|Setspawning false)
  (Variables|Default|Setdied true)
  (Transformation|SetActorLocation "0.000000,0.000000,-250.000000" false false))

(event Custom|AttackEvent
  (if (Math|Random|RandomBool)
    (bind _returnvalue (Animation|PlayAnimMontage "/Game/Asset/Goblin/Animations/Anim_Attack1_Montage.Anim_Attack1_Montage" 1.0 "None"))
    (Utilities|FlowControl|Delay _returnvalue)
    (else
      (bind _returnvalue_2 (Animation|PlayAnimMontage "/Game/Asset/Goblin/Animations/Anim_Attack2_Montage.Anim_Attack2_Montage" 1.0 "None"))
      (Utilities|FlowControl|Delay _returnvalue_2)))
  (Variables|Default|Setattacking false))

(event EventBeginPlay)

(fn ConstructionScript
  (|CallParentFunction))

(fn Die
  (|CallParentFunction)
  (CallFunction|DieEvent))

(fn SpawnObstacle
  (params (location :type Vector)))

(fn ResetPosition
  (params (location :type Vector :default "0, 0, 0"))
  (|CallParentFunction location)
  (Variables|Default|Setpath (Variables|Default|GetpathOri)))

(fn SubExplodeTime)

(fn Attack
  (params (AttackedActor :type Actor%20Object%20Reference))
  (|CallParentFunction AttackedActor)
  (CallFunction|AttackEvent))

(fn BombExplode
  (params (cells :type Array%20of%20BP%20Cell%20Object%20References) (mazeSize :type Int%20Point%20Structure) (gridSize :type Integer))
  (bind _returnvalue (/ gridSize 2))
  (bind _returnvalue_2 (Math|Conversions|ToFloat(Integer) _returnvalue))
  (|CallParentFunction cells "" 0)
  (Utilities|Array|Insert (Variables|Default|Getpath) (Variables|Default|Getlocation))
  (Variables|Default|Setlocation (Utilities|Array|Get(acopy) (Variables|Default|GetpathOri) (Utilities|Operators|Subtract (Utilities|Array|Length (Variables|Default|GetpathOri)) (Utilities|Array|Length (Variables|Default|Getpath)) 2)))
  (CallFunction|FlyEvent (+ (Transformation|GetActorLocation (Utilities|Array|Get(acopy) cells (CallFunction|GetIndex (Variables|Default|Getlocation) mazeSize))) (Math|Vector|MakeVector _returnvalue_2 _returnvalue_2 0.0))))

(fn Destroy
  (bind _obstacle (Variables|Default|Getobstacle))
  (|CallParentFunction)
  (Utilities|IsValid _obstacle
    (:Is%20Valid
      (Actor|DestroyActor _obstacle))
    (:Is%20Not%20Valid
      _))
  (Actor|DestroyActor))

(fn Move
  (params (cells :type Array%20of%20BP%20Cell%20Object%20References) (mazeSize :type Int%20Point%20Structure) (gridSize :type Integer) (playerLoc :type Int%20Point%20Structure))
  (|CallParentFunction cells mazeSize gridSize playerLoc)
  (CallFunction|MoveEvent cells mazeSize gridSize playerLoc)
  (return))