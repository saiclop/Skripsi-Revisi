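; Maze disturber NPC that hides its mesh and spawns a timed BP_Bomb as its obstacle.
; Initialize caches the obstacle cell, its four grid neighbours and their original wall arrays.
; When SubExplodeTime reports an explosion, it flags the cell and, if walls are present, clears its wall visuals and rebuilds the neighbours' facing sides.
; ResetPosition shows the NPC again, destroys the bomb and restores cached walls if the timer had run out.
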(event EventBeginPlay
  (|CallParentFunction))

(event Collision|EventActorBeginOverlap
  (params (OtherActor :type Actor%20Object%20Reference))
  (|CallParentFunction OtherActor) ; This node is disabled and will not be called.\nDrag off pins to build functionality.
)

(event EventTick
  (params (DeltaSeconds :type Float%20%28single-precision%29))
  (|CallParentFunction DeltaSeconds) ; This node is disabled and will not be called.\nDrag off pins to build functionality.
)

(fn ConstructionScript
  (|CallParentFunction)
  (Variables|Default|Setpower 2))

(fn SpawnObstacle
  (params (location :type Vector :default "0, 0, 0"))
  (|CallParentFunction location)
  (Rendering|SetVisibility (Variables|Default|GetStaticMesh) false false)
  (bind _returnvalue (Game|SpawnActorfromClass "/Game/Skripsi/Blueprints/Obstacle/BP_Bomb.BP_Bomb_C" (Math|Transform|MakeTransform location "0, 0, 0" "1.000000,1.000000,1.000000") "AlwaysSpawn" 0 0))
  (Default|SetExplodeTime _returnvalue (Variables|Default|GetbombExplodeTime))
  (Variables|Default|Setobstacle _returnvalue))

(fn SubExplodeTime
  (bind _obstaclecell (Variables|Default|GetobstacleCell))
  (bind _cellstrbl (Variables|Default|GetcellsTRBL))
  (bind _cellstrbl_2 (Variables|Default|GetcellsTRBL))
  (bind _cellstrbl_3 (Variables|Default|GetcellsTRBL))
  (bind _cellstrbl_4 (Variables|Default|GetcellsTRBL))
  (bind _output (Utilities|Array|Get(acopy) _cellstrbl 3))
  (bind _output_2 (Utilities|Array|Get(acopy) _cellstrbl_2))
  (bind _output_3 (Utilities|Array|Get(acopy) _cellstrbl_3 1))
  (bind _output_4 (Utilities|Array|Get(acopy) _cellstrbl_4 2))
  (bind _wall (Variables|/Game/Skripsi/Blueprints/Maze/BP_Cell.BP_Cell_C|Getwall _obstaclecell))
  (|CallParentFunction)
  (bind _asbp_bomb (Utilities|Casting|CastToBP_Bomb (Variables|Default|Getobstacle)))
  (bind (_explode _haswall) (Default|SubExplodeTime _asbp_bomb _wall (Variables|/Game/Skripsi/Blueprints/Maze/BP_Cell.BP_Cell_C|GetwallVisualize _obstaclecell)))
  (if _explode
    (Variables|/Game/Skripsi/Blueprints/Maze/BP_Cell.BP_Cell_C|Setexplode (Variables|Default|GetobstacleCell) true)
    (if _haswall
      (for (_ _array_index) _wall
        (Utilities|Array|SetArrayElem _wall _array_index true))
      (Default|RemoveWall (Variables|Default|GetobstacleCell))
      (Utilities|FlowControl|Sequence
        (:then_0
          ;[1 1 1] atas
          (Utilities|IsValid _output_2
            (:Is%20Valid
              (Utilities|Array|SetArrayElem (Variables|/Game/Skripsi/Blueprints/Maze/BP_Cell.BP_Cell_C|Getwall _output_2) 2 true)
              (Utilities|Array|SetArrayElem (Variables|/Game/Skripsi/Blueprints/Maze/BP_Cell.BP_Cell_C|GetwallVisualize _output_2) 2 false)
              (Default|RemoveWall _output_2)
              (Default|GenerateWall _output_2))))
        (:then_1
          ;[1 1 1] kanan
          (Utilities|IsValid _output_3
            (:Is%20Valid
              (Utilities|Array|SetArrayElem (Variables|/Game/Skripsi/Blueprints/Maze/BP_Cell.BP_Cell_C|Getwall _output_3) 3 true)
              (Utilities|Array|SetArrayElem (Variables|/Game/Skripsi/Blueprints/Maze/BP_Cell.BP_Cell_C|GetwallVisualize _output_3) 3 false)
              (Default|RemoveWall _output_3)
              (Default|GenerateWall _output_3))))
        (:then_2
          ;[1 1 1] bawah
          (Utilities|IsValid _output_4
            (:Is%20Valid
              (Utilities|Array|SetArrayElem (Variables|/Game/Skripsi/Blueprints/Maze/BP_Cell.BP_Cell_C|Getwall _output_4) 0 true)
              (Utilities|Array|SetArrayElem (Variables|/Game/Skripsi/Blueprints/Maze/BP_Cell.BP_Cell_C|GetwallVisualize _output_4) 0 false)
              (Default|RemoveWall _output_4)
              (Default|GenerateWall _output_4))))
        (:then_3
          ;[1 1 1] kiri
          (Utilities|IsValid _output
            (:Is%20Valid
              (Utilities|Array|SetArrayElem (Variables|/Game/Skripsi/Blueprints/Maze/BP_Cell.BP_Cell_C|Getwall _output) 1 true)
              (Utilities|Array|SetArrayElem (Variables|/Game/Skripsi/Blueprints/Maze/BP_Cell.BP_Cell_C|GetwallVisualize _output) 1 false)
              (Default|RemoveWall _output)
              (Default|GenerateWall _output))))))))

(fn ResetPosition
  (params (location :type Vector :default "0, 0, 0"))
  (bind _obstaclecell (Variables|Default|GetobstacleCell))
  (bind _wallvisualize (Variables|/Game/Skripsi/Blueprints/Maze/BP_Cell.BP_Cell_C|GetwallVisualize _obstaclecell))
  (|CallParentFunction location)
  (Utilities|IsValid (Variables|Default|Getobstacle)
    (:Is%20Valid
      (Rendering|SetVisibility (Variables|Default|GetStaticMesh) true false)
      (bind _asbp_bomb (Utilities|Casting|CastToBP_Bomb (Variables|Default|Getobstacle)))
      (if (> (Variables|/Game/Skripsi/Blueprints/Obstacle/BP_Bomb.BP_Bomb_C|GetexplodeTime _asbp_bomb) 0)
        (Actor|DestroyActor (Variables|Default|Getobstacle))
        (else
          (Variables|/Game/Skripsi/Blueprints/Maze/BP_Cell.BP_Cell_C|Setexplode (Variables|Default|GetobstacleCell) false)
          (for (_array_element _array_index) (Variables|Default|GetcellsTRBL)
            (Utilities|IsValid _array_element
              (:Is%20Valid
                (Variables|/Game/Skripsi/Blueprints/Maze/BP_Cell.BP_Cell_C|Setwall _array_element (.array (Utilities|Array|Get(acopy) (Variables|Default|Getwalls) _array_index)))
                (for (_ _array_index_2) (Variables|/Game/Skripsi/Blueprints/Maze/BP_Cell.BP_Cell_C|GetwallVisualize _array_element)
                  (Utilities|Array|SetArrayElem (Variables|/Game/Skripsi/Blueprints/Maze/BP_Cell.BP_Cell_C|GetwallVisualize _array_element) _array_index_2 true))
                (Default|RemoveWall _array_element)
                (Default|GenerateWall _array_element))))
          (Variables|/Game/Skripsi/Blueprints/Maze/BP_Cell.BP_Cell_C|Setwall _obstaclecell (Variables|Default|GetwallOri))
          (for (_ _array_index_3) _wallvisualize
            (Utilities|Array|SetArrayElem _wallvisualize _array_index_3 true))
          (Default|RemoveWall _obstaclecell)
          (Default|GenerateWall _obstaclecell)
          (Actor|DestroyActor (Variables|Default|Getobstacle)))))))

(fn Initialize
  (params (cells :type Array%20of%20BP%20Cell%20Object%20References) (mazeSize :type Int%20Point%20Structure))
  (bind _obstaclelocation (Variables|Default|GetobstacleLocation))
  (bind _obstaclelocation_2 (Variables|Default|GetobstacleLocation))
  (bind _obstaclelocation_3 (Variables|Default|GetobstacleLocation))
  (bind _obstaclelocation_4 (Variables|Default|GetobstacleLocation))
  (bind _obstaclelocation_5 (Variables|Default|GetobstacleLocation))
  (bind _index (CallFunction|GetIndex _obstaclelocation_5 mazeSize))
  (bind _returnvalue (+ (.x _obstaclelocation_2) 1))
  (bind _returnvalue_2 (+ (.y _obstaclelocation_3) 1))
  (bind _returnvalue_3 (- (.y _obstaclelocation) 1))
  (bind _returnvalue_4 (- (.x _obstaclelocation_4) 1))
  (bind _index_2 (CallFunction|GetIndex (Utilities|Struct|MakeIntPoint _returnvalue_4 (.y _obstaclelocation_4)) mazeSize))
  (bind _index_3 (CallFunction|GetIndex (Utilities|Struct|MakeIntPoint (.x _obstaclelocation) _returnvalue_3) mazeSize))
  (bind _index_4 (CallFunction|GetIndex (Utilities|Struct|MakeIntPoint _returnvalue (.y _obstaclelocation_2)) mazeSize))
  (bind _index_5 (CallFunction|GetIndex (Utilities|Struct|MakeIntPoint (.x _obstaclelocation_3) _returnvalue_2) mazeSize))
  (bind _output (Utilities|Array|Get(acopy) cells _index))
  (bind _output_2 (Utilities|Array|Get(acopy) cells _index_3))
  (bind _output_3 (Utilities|Array|Get(acopy) cells _index_4))
  (bind _output_4 (Utilities|Array|Get(acopy) cells _index_5))
  (bind _output_5 (Utilities|Array|Get(acopy) cells _index_2))
  (|CallParentFunction cells mazeSize)
  (Utilities|FlowControl|Sequence
    (:then_0
      ;[1 1 1] resize
      (Utilities|Array|Resize (Variables|Default|GetcellsTRBL) 4)
      (Utilities|Array|Resize (Variables|Default|Getwalls) 4))
    (:then_1
      ;[1 1 1] atas obstacle cell
      (if (> (.y (Variables|Default|GetobstacleLocation)) 0)
        (Utilities|Array|SetArrayElem (Variables|Default|GetcellsTRBL) 0 _output_2)
        (Utilities|Array|SetArrayElem (Variables|Default|Getwalls) 0 (Utilities|Struct|MakeS_ArrayBool (Variables|/Game/Skripsi/Blueprints/Maze/BP_Cell.BP_Cell_C|Getwall _output_2)))))
    (:then_2
      ;[1 1 1] kanan obstacle cell
      (if (< (.x (Variables|Default|GetobstacleLocation)) (- (.x mazeSize) 1))
        (Utilities|Array|SetArrayElem (Variables|Default|GetcellsTRBL) 1 _output_3)
        (Utilities|Array|SetArrayElem (Variables|Default|Getwalls) 1 (Utilities|Struct|MakeS_ArrayBool (Variables|/Game/Skripsi/Blueprints/Maze/BP_Cell.BP_Cell_C|Getwall _output_3)))))
    (:then_3
      ;[1 1 1] bawah obstacle cell
      (if (< (.y (Variables|Default|GetobstacleLocation)) (- (.y mazeSize) 1))
        (Utilities|Array|SetArrayElem (Variables|Default|GetcellsTRBL) 2 _output_4)
        (Utilities|Array|SetArrayElem (Variables|Default|Getwalls) 2 (Utilities|Struct|MakeS_ArrayBool (Variables|/Game/Skripsi/Blueprints/Maze/BP_Cell.BP_Cell_C|Getwall _output_4)))))
    (:then_4
      ;[1 1 1] kiri obstacle cell
      (if (> (.x (Variables|Default|GetobstacleLocation)) 0)
        (Utilities|Array|SetArrayElem (Variables|Default|GetcellsTRBL) 3 _output_5)
        (Utilities|Array|SetArrayElem (Variables|Default|Getwalls) 3 (Utilities|Struct|MakeS_ArrayBool (Variables|/Game/Skripsi/Blueprints/Maze/BP_Cell.BP_Cell_C|Getwall _output_5)))))
    (:then_5
      ;[1 1 1] obstacle cell
      (Variables|Default|SetobstacleCell _output)
      (Variables|Default|SetwallOri (Variables|/Game/Skripsi/Blueprints/Maze/BP_Cell.BP_Cell_C|Getwall _output)))))