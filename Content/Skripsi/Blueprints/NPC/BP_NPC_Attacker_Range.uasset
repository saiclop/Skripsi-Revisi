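; Skeleton attacker NPC for a grid maze, armed with a sword or bow according to its Movement setting.
; SetMovement swaps weapon visibility and anim class (Horizontal sword, Vertical bow), while construction makes armor parts follow the body mesh pose.
; CanAttack allows hits on its own cell or an adjacent, unwalled one.
; Attack and Die overrides play weapon-specific montages, clearing state flags afterward; death also moves the actor below the origin.
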(event Custom|DieEvent
  (Utilities|FlowControl|Delay 0.3)
  (switch Utilities|FlowControl|Switch|SwitchonEMovementPriority (Variables|Default|Getmovement)
    (:Horizontal
      (bind _returnvalue (Animation|PlayAnimMontage "/Game/Asset/Skeleton/Animations/Anim_Death_Sword_Montage.Anim_Death_Sword_Montage" 1.0 "None"))
      (Utilities|FlowControl|Delay (- _returnvalue 0.1))
      (Transformation|SetActorLocation "0.000000,0.000000,-250.000000" false false))
    (:Vertical
      (bind _returnvalue_2 (Animation|PlayAnimMontage "/Game/Asset/Skeleton/Animations/Anim_Death_Bow_Montage.Anim_Death_Bow_Montage" 1.0 "None"))
      (Utilities|FlowControl|Delay (- _returnvalue_2 0.1))
      (Transformation|SetActorLocation "0.000000,0.000000,-250.000000" false false)))
  (Variables|Default|Setdying false))

(event Custom|AttackEvent
  (switch Utilities|FlowControl|Switch|SwitchonEMovementPriority (Variables|Default|Getmovement)
    (:Horizontal
      (if (Math|Random|RandomBool)
        (bind _returnvalue (Animation|PlayAnimMontage "/Game/Asset/Skeleton/Animations/Anim_Attack_Sword_1_Montage.Anim_Attack_Sword_1_Montage" 1.0 "None"))
        (Utilities|FlowControl|Delay _returnvalue)
        (else
          (bind _returnvalue_2 (Animation|PlayAnimMontage "/Game/Asset/Skeleton/Animations/Anim_Attack_Sword_2_Montage.Anim_Attack_Sword_2_Montage" 1.0 "None"))
          (Utilities|FlowControl|Delay _returnvalue_2))))
    (:Vertical
      (bind _returnvalue_3 (Animation|PlayAnimMontage "/Game/Asset/Skeleton/Animations/Anim_Attack_Montage.Anim_Attack_Montage" 1.0 "None"))
      (Utilities|FlowControl|Delay _returnvalue_3)))
  (Variables|Default|Setattacking false))

(event EventBeginPlay
  (|CallParentFunction) ; This node is disabled and will not be called.\nDrag off pins to build functionality.
)

(event Collision|EventActorBeginOverlap
  (params (OtherActor :type Actor%20Object%20Reference))
  (|CallParentFunction OtherActor) ; This node is disabled and will not be called.\nDrag off pins to build functionality.
)

(event EventTick
  (params (DeltaSeconds :type Float%20%28single-precision%29))
  (|CallParentFunction DeltaSeconds) ; This node is disabled and will not be called.\nDrag off pins to build functionality.
)

(fn ConstructionScript
  (|CallParentFunction)
  (Components|SkinnedMesh|SetLeaderPoseComponent (Variables|Default|GetSK_HelmetPart) (Variables|Character|GetMesh) false false)
  (CallFunction|SetMovement (Variables|Default|Getmovement))
  (Variables|Default|Setpower 4))

(fn SetMovement
  (params (movement :type EMovementPriority%20Enum :default "Horizontal"))
  (|CallParentFunction movement)
  (switch Utilities|FlowControl|Switch|SwitchonEMovementPriority movement
    (:Horizontal
      (Rendering|SetVisibility (Variables|Default|GetSK_Bow) false true)
      (Rendering|SetVisibility (Variables|Default|GetSM_ArrowCut) false true)
      (Rendering|SetVisibility (Variables|Default|GetSM_Sword) true false)
      (Class|SkeletalMeshComponent|SetAnimClass (Variables|Character|GetMesh) "/Game/Asset/Skeleton/Animations/ABP_SwordSkeleton.ABP_SwordSkeleton_C"))
    (:Vertical
      (Rendering|SetVisibility (Variables|Default|GetSK_Bow) true true)
      (Rendering|SetVisibility (Variables|Default|GetSM_ArrowCut) true true)
      (Rendering|SetVisibility (Variables|Default|GetSM_Sword) false false)
      (Class|SkeletalMeshComponent|SetAnimClass (Variables|Character|GetMesh) "/Game/Asset/Skeleton/Animations/ABP_BowSkeleton.ABP_BowSkeleton_C"))))

(fn CanAttack?
  (params (playerLocation :type Int%20Point%20Structure) (cells :type Array%20of%20BP%20Cell%20Object%20References) (mazeSize :type Int%20Point%20Structure))
  (bind _location (Variables|Default|Getlocation))
  (bind _location_2 (Variables|Default|Getlocation))
  (bind _location_3 (Variables|Default|Getlocation))
  (bind _location_4 (Variables|Default|Getlocation))
  (if (Math|Boolean|ORBoolean (Class|KismetMathLibrary|EqualIntPointIntPoint playerLocation (Variables|Default|Getlocation)) (Math|Boolean|ANDBoolean (== (.x playerLocation) (.x _location)) (== (.y playerLocation) (+ (.y _location) -1)) (not (Utilities|Array|Get(acopy) (Variables|/Game/Skripsi/Blueprints/Maze/BP_Cell.BP_Cell_C|Getwall (Utilities|Array|Get(acopy) cells (CallFunction|GetIndex (Variables|Default|Getlocation) mazeSize)))))) (Math|Boolean|ANDBoolean (== (.x playerLocation) (.x _location_2)) (== (.y playerLocation) (+ (.y _location_2) 1)) (not (Utilities|Array|Get(acopy) (Variables|/Game/Skripsi/Blueprints/Maze/BP_Cell.BP_Cell_C|Getwall (Utilities|Array|Get(acopy) cells (CallFunction|GetIndex (Variables|Default|Getlocation) mazeSize))) 2))) (Math|Boolean|ANDBoolean (== (.x playerLocation) (+ (.x _location_3) 1)) (== (.y playerLocation) (.y _location_3)) (not (Utilities|Array|Get(acopy) (Variables|/Game/Skripsi/Blueprints/Maze/BP_Cell.BP_Cell_C|Getwall (Utilities|Array|Get(acopy) cells (CallFunction|GetIndex (Variables|Default|Getlocation) mazeSize))) 1))) (Math|Boolean|ANDBoolean (== (.x playerLocation) (+ (.x _location_4) -1)) (== (.y playerLocation) (.y _location_4)) (not (Utilities|Array|Get(acopy) (Variables|/Game/Skripsi/Blueprints/Maze/BP_Cell.BP_Cell_C|Getwall (Utilities|Array|Get(acopy) cells (CallFunction|GetIndex (Variables|Default|Getlocation) mazeSize))) 3))))
    (return true)
    (else
      (return false))))

(fn Die
  (|CallParentFunction)
  (CallFunction|DieEvent))

(fn Attack
  (params (AttackedActor :type Actor%20Object%20Reference))
  (|CallParentFunction AttackedActor)
  (CallFunction|AttackEvent))