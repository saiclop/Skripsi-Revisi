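; Melee zombie NPC for a grid maze, which can attack only when the player occupies its own cell and has a Power of 3.
; Movement axis (horizontal or vertical) selects the zombie material at construction.
; Attack and Die extend the parent with montage-timed events that clear the Attacking or Dying flag, playing a random attack or hiding the body below the map after death.
; The player reset-position binding is unconnected.
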(event Custom|DieEvent
  (Utilities|FlowControl|Delay 0.3)
  (bind _returnvalue (Animation|PlayAnimMontage "/Game/Asset/Zombie/Animations/Anim_Death_Montage.Anim_Death_Montage" 1.0 "None"))
  (Utilities|FlowControl|Delay (- _returnvalue 0.1))
  (Transformation|SetActorLocation "0.000000,0.000000,-250.000000" false false)
  (Variables|Default|Setdying false))

(event Custom|AttackEvent
  (if (Math|Random|RandomBool)
    (bind _returnvalue (Animation|PlayAnimMontage "/Game/Asset/Zombie/Animations/Anim_Attack1_Montage.Anim_Attack1_Montage" 1.0 "None"))
    (Utilities|FlowControl|Delay _returnvalue)
    (else
      (bind _returnvalue_2 (Animation|PlayAnimMontage "/Game/Asset/Zombie/Animations/Anim_Attack2_Montage.Anim_Attack2_Montage" 1.0 "None"))
      (Utilities|FlowControl|Delay _returnvalue_2)))
  (Variables|Default|Setattacking false))

(event Custom|ResetPosition_Event
  (CallFunction|FlyEvent "0, 0, 0"))

(event EventBeginPlay
  (|CallParentFunction))

(event Collision|EventActorBeginOverlap
  (params (OtherActor :type Actor%20Object%20Reference))
  (|CallParentFunction OtherActor) ; This node is disabled and will not be called.\nDrag off pins to build functionality.
)

(event EventTick
  (params (DeltaSeconds :type Float%20%28single-precision%29))
  (|CallParentFunction DeltaSeconds) ; This node is disabled and will not be called.\nDrag off pins to build functionality.
)

(fn ConstructionScript
  (|CallParentFunction)
  (CallFunction|SetMovement (Variables|Default|Getmovement))
  (Variables|Default|Setpower 3))

(fn SetMovement
  (params (movement :type EMovementPriority%20Enum :default "Horizontal"))
  (|CallParentFunction movement)
  (switch Utilities|FlowControl|Switch|SwitchonEMovementPriority movement
    (:Horizontal
      (Rendering|Material|SetMaterial (Variables|Character|GetMesh) 0 "/Game/Asset/Zombie/Materials/MI_Zombie_1.MI_Zombie_1"))
    (:Vertical
      (Rendering|Material|SetMaterial (Variables|Character|GetMesh) 0 "/Game/Asset/Zombie/Materials/MI_Zombie_2.MI_Zombie_2"))))

(fn CanAttack?
  (params (playerLocation :type Int%20Point%20Structure) (cells :type Array%20of%20BP%20Cell%20Object%20References) (mazeSize :type Int%20Point%20Structure))
  (if (Class|KismetMathLibrary|EqualIntPointIntPoint playerLocation (Variables|Default|Getlocation))
    (return true)
    (else
      (return false))))

(fn Die
  (|CallParentFunction)
  (CallFunction|DieEvent))

(fn Attack
  (params (AttackedActor :type Actor%20Object%20Reference))
  (|CallParentFunction AttackedActor)
  (CallFunction|AttackEvent))