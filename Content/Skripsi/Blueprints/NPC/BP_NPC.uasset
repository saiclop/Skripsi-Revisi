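; Base NPC Blueprint for a maze game, holding shared state flags for moving, attacking and dying.
; Attack turns it toward its target, Die sets death flags, and ResetPosition clears movement and death state and repositions it.
; FlyEvent uses a timeline to lerp it to a point raised above a given location.
; Initialize, Move and Destroy are empty stubs, and BombExplode only checks for death.
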(event Custom|FlyEvent
  (params (Location :type Vector))
  (Variables|Default|SetstartLoc (Transformation|GetActorLocation))
  (bind _alpha (Timeline|Fly PlayFromStart)
    (:Update
      (Transformation|SetActorLocation (Math|Vector|Lerp(Vector) (Variables|Default|GetstartLoc) (+ Location "0.000000,0.000000,200.000000") _alpha) false false))))

(event EventBeginPlay)

(event Collision|EventActorBeginOverlap
  (params (OtherActor :type Actor%20Object%20Reference)))

(event EventTick
  (params (DeltaSeconds :type Float%20%28single-precision%29)))

(fn ConstructionScript)

(fn Attack
  (params (AttackedActor :type Actor%20Object%20Reference))
  (Variables|Default|Setattacking true)
  (Transformation|SetActorRotation (Math|Rotator|FindLookatRotation (Transformation|GetActorLocation) (Transformation|GetActorLocation AttackedActor))))

(fn Die
  (Variables|Default|Setdying true)
  (Variables|Default|Setdied true))

(fn ResetPosition
  (params (location :type Vector))
  (Variables|Default|Setmoving false)
  (Variables|Default|Setdied false)
  (Variables|Default|Setlocation (Variables|Default|GetspawnLocation))
  (Transformation|SetActorLocationAndRotation location "0.000000,90.000000,0.000000"))

(fn Initialize
  (params (cells :type Array%20of%20BP%20Cell%20Object%20References) (mazeSize :type Int%20Point%20Structure)))

(fn BombExplode
  (params (cells :type Array%20of%20BP%20Cell%20Object%20References) (mazeSize :type Int%20Point%20Structure) (gridSize :type Integer))
  (if (Variables|Default|Getdied)
    (return)))

(fn Destroy)

(fn Move
  (params (cells :type Array%20of%20BP%20Cell%20Object%20References) (mazeSize :type Int%20Point%20Structure) (gridSize :type Integer) (playerLoc :type Int%20Point%20Structure)))